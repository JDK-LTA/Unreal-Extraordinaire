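; BossAIController is the AI controller for a boss enemy, setting up its blackboard and starting its behavior tree.
; On BeginPlay it activates BossBB, resets the spawned-eye count, and stores the player reference, the player's initial location and a Monstro tear count.
; It then runs BossBT, but only if the player character casts to PlayerBP.
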(event EventBeginPlay
  (bind _returnvalue (Game|GetPlayerCharacter 0))
  (bind _blackboardcomponent (Class|AIController|UseBlackboard "/Game/Blueprints/Enemies/BossBB.BossBB"))
  (Class|BlackboardComponent|SetValueasInt _blackboardcomponent (Variables|Default|GetK_NumOfSpawnedEyes))
  (bind _asplayer_bp (Utilities|Casting|CastToPlayerBP _returnvalue))
  (AI|Components|Blackboard|SetValueasObject _blackboardcomponent (Variables|Default|GetK_Player) _asplayer_bp)
  (AI|Components|Blackboard|SetValueasVector _blackboardcomponent (Variables|Default|GetK_TargetLocation) (Transformation|GetActorLocation _returnvalue))
  (Class|BlackboardComponent|SetValueasInt _blackboardcomponent (Variables|Default|GetK_NumOfMonstroTears) 10)
  (AI|RunBehaviorTree "/Game/Blueprints/Enemies/BossBT.BossBT"))

(fn ConstructionScript)