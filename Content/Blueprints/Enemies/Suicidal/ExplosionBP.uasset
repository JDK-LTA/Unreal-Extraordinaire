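; ExplosionBP is a one-shot explosion actor under the suicidal enemy assets that damages the player on spawn.
; On BeginPlay it plays an attenuated sound, fires a RadialForce impulse and sphere-overlaps pawns filtered to PlayerBP, drawing a debug sphere.
; The first player found receives DamageMe with Damage falling off linearly with distance over Radius.
; The actor destroys itself when its particle system finishes.
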(event OnSystemFinished(ParticleSystem)
  (params (PSystem :type Particle%20System%20Component%20Object%20Reference))
  (Actor|DestroyActor))

(event EventBeginPlay
  (bind _returnvalue (Transformation|GetActorLocation))
  (bind _radius (Variables|Default|GetRadius))
  (Audio|PlaySoundatLocation "/Game/SciFiWeapDark/Sound/GrenadeLauncher/GrenadeLauncher_Explosion_Cue.GrenadeLauncher_Explosion_Cue" _returnvalue "0, 0, 0" 1.0 1.0 0.0 "/Game/SciFiWeapDark/Sound/Attenuation/Explosion_att.Explosion_att" 0 0)
  (Class|RadialForceComponent|FireImpulse (Variables|Default|GetRadialForce))
  (bind _outactors (Collision|SphereOverlapActors _returnvalue _radius (Variables|Default|GetPawnType) "/Game/Blueprints/PlayerBPs/PlayerBP.PlayerBP_C"))
  (Rendering|Debug|DrawDebugSphere _returnvalue _radius 12 "(R=1.000000,G=1.000000,B=1.000000,A=1.000000)" 5.0)
  (bind _asplayer_bp (Utilities|Casting|CastToPlayerBP (Utilities|Array|Get(acopy) _outactors)))
  (Default|DamageMe _asplayer_bp (* (- 1.0 (/ (Math|Vector|Distance(Vector) _returnvalue (Transformation|GetActorLocation _asplayer_bp)) (Variables|Default|GetRadius))) (Variables|Default|GetDamage))))

(fn ConstructionScript)