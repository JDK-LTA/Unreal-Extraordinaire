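; OrbBP is an orb pickup that randomly becomes good (green) or evil (red) on BeginPlay.
; When an EnemyBase overlaps its Box, a good orb restores a tenth of that enemy's missing HP, while an evil one damages the player character.
; A PlayerBP overlap passes negative damage to DamageMe regardless of type.
; The orb is not destroyed or disabled after an overlap.
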(event OnComponentBeginOverlap(Box)
  (params (OverlappedComponent :type Primitive%20Component%20Object%20Reference) (OtherActor :type Actor%20Object%20Reference) (OtherComp :type Primitive%20Component%20Object%20Reference) (OtherBodyIndex :type Integer) (bFromSweep :type Boolean) (SweepResult :type Hit%20Result%20Structure%20%28by%20ref%29))
  (bind _asenemy_base (Utilities|Casting|CastToEnemyBase OtherActor)
    (:then
      (if (Variables|Default|GetGoodTrue-EvilFalse)
        (Variables|/Game/Blueprints/Enemies/Boss/EnemyBase.EnemyBase_C|SetCurrentHP _asenemy_base (+ (* (- 1.0 (/ (Variables|/Game/Blueprints/Enemies/Boss/EnemyBase.EnemyBase_C|GetCurrentHP _asenemy_base) (Variables|/Game/Blueprints/Enemies/Boss/EnemyBase.EnemyBase_C|GetMaxHP _asenemy_base))) 0.1 (Variables|/Game/Blueprints/Enemies/Boss/EnemyBase.EnemyBase_C|GetMaxHP _asenemy_base)) (Variables|/Game/Blueprints/Enemies/Boss/EnemyBase.EnemyBase_C|GetCurrentHP _asenemy_base)))
        (else
          (bind _asplayer_bp (Utilities|Casting|CastToPlayerBP (Game|GetPlayerCharacter 0)))
          (Default|DamageMe _asplayer_bp 1e+01))))
    (:CastFailed
      (bind _asplayer_bp_2 (Utilities|Casting|CastToPlayerBP OtherActor))
      (Default|DamageMe _asplayer_bp_2 -1e+01))))

(event EventBeginPlay
  (bind _cube2 (Variables|Default|GetCube2))
  (bind _output_get (Variables|Default|SetGoodTrue-EvilFalse (Math|Random|RandomBool)))
  (if _output_get
    (Rendering|Material|SetMaterial _cube2 0 "/Game/Materials/Green.Green")
    (else
      (Rendering|Material|SetMaterial _cube2 0 "/Game/Materials/Red.Red"))))

(fn ConstructionScript)