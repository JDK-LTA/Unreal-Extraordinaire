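; PlopEyeBP is an eye enemy that moves by projectile movement and redirects itself toward the player when it bounces.
; On each bounce, LookForPlayer runs a Camera-channel line trace to the player character, with debug drawing and log prints.
; If the trace hits PlayerBP, SetDirToPlayer sets velocity to the unnormalized offset toward the player times InitialSpeed, so speed scales with distance.
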(event OnProjectileBounce(ProjectileMovement)
  (params (ImpactResult :type Hit%20Result%20Structure%20%28by%20ref%29) (ImpactVelocity :type Vector%20%28by%20ref%29 :default "0, 0, 0"))
  (bind _success (CallFunction|LookforPlayer))
  (if _success
    (CallFunction|SetDirtoPlayer)))

(fn ConstructionScript)

(fn LookforPlayer
  (Development|PrintString "Looking for player")
  (bind _outhit (Collision|LineTraceByChannel (Transformation|GetActorLocation) (Transformation|GetActorLocation (Game|GetPlayerCharacter 0)) "TraceTypeQuery2" false 0 "ForDuration"))
  (Utilities|Casting|CastToPlayerBP (.HitActor (Collision|BreakHitResult _outhit))
    (:then
      (return true))
    (:CastFailed
      (Development|PrintString "Nope")
      (return false))))

(fn SetDirtoPlayer
  (bind _projectilemovement (Variables|Default|GetProjectileMovement))
  (bind _output_get (Variables|Default|SetTargetDirection (- (Transformation|GetActorLocation (Game|GetPlayerCharacter 0)) (Transformation|GetActorLocation))))
  (Variables|/Script/Engine.MovementComponent|SetVelocity _projectilemovement (* _output_get (Variables|/Script/Engine.ProjectileMovementComponent|GetInitialSpeed _projectilemovement))))