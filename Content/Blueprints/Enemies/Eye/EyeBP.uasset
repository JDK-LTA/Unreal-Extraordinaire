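; EyeBP is an enemy that flies in a straight line at the player, deals damage on capsule contact and then destroys itself.
; BeginPlay aims at the player and starts a looping timer that moves it with swept transforms, scaled by speed and frame delta time rather than timer interval.
; Hitting anything else triggers a visibility line trace, re-aiming if the player is seen or zeroing its direction otherwise.
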(event OnComponentHit(CapsuleComponent)
  (params (HitComponent :type Primitive%20Component%20Object%20Reference) (OtherActor :type Actor%20Object%20Reference) (OtherComp :type Primitive%20Component%20Object%20Reference) (NormalImpulse :type Vector :default "0, 0, 0") (Hit :type Hit%20Result%20Structure%20%28by%20ref%29))
  (bind _asplayer_bp (Utilities|Casting|CastToPlayerBP OtherActor)
    (:then
      (Variables|/Game/Blueprints/PlayerBPs/PlayerBP.PlayerBP_C|SetCurrentHP _asplayer_bp (- (Variables|/Game/Blueprints/PlayerBPs/PlayerBP.PlayerBP_C|GetCurrentHP _asplayer_bp) 5.0))
      (Actor|DestroyActor))
    (:CastFailed
      (bind _success (CallFunction|LookforPlayer))
      (if _success
        (CallFunction|SetTargetDirtoPlayer)
        (else
          (Variables|Default|SetTargetDirection "0, 0, 0"))))))

(event Custom|MoveTowards
  (bind _mesh (Variables|Character|GetMesh))
  (bind _returnvalue (Transformation|GetWorldTransform _mesh))
  (Transformation|SetActorTransform (Math|Transform|MakeTransform (+ (.location _returnvalue) (* (Math|Vector|Normalize (Variables|Default|GetTargetDirection)) (* (Utilities|Time|GetWorldDeltaSeconds) (Variables|Default|GetSpeed)))) (.rotation _returnvalue) (.scale _returnvalue)) true))

(event EventBeginPlay
  (CallFunction|SetTargetDirtoPlayer)
  (Utilities|Time|SetTimerbyEvent (delegate Custom|MoveTowards) 0.05 true))

(fn ConstructionScript)

(fn LookforPlayer
  (bind _outhit (Collision|LineTraceByChannel (Transformation|GetActorLocation) (Transformation|GetActorLocation (Game|GetPlayerCharacter 0)) "TraceTypeQuery1" false 0 "None"))
  (Utilities|Casting|CastToPlayerBP (.HitActor (Collision|BreakHitResult _outhit))
    (:then
      (return true))
    (:CastFailed
      (return false))))

(fn SetTargetDirtoPlayer
  (Variables|Default|SetTargetDirection (- (Transformation|GetActorLocation (Game|GetPlayerCharacter 0)) (Transformation|GetActorLocation))))