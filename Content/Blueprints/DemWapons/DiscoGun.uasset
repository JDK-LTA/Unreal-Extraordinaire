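; DiscoGun is a weapon Blueprint with an automatic primary fire and a charged secondary fire.
; Primary fires a DamageBouncy projectile on pull, then repeats via a looping RoF timer until release, with a DoOnce limiting re-press spam.
; Secondary runs the DiscoDamage timeline and launches a DiscoSpawner on release or completion, copying the timeline's truncated value into its Damage.
; A second DoOnce holds secondary shots to a one-second cooldown.
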(event Custom|Fire
  (CallFunction|Proyectile 0.0 "/Game/Blueprints/DemWapons/Proyectiles/DamageBouncy.DamageBouncy_C")
  (Utilities|FlowControl|Delay (Variables|Default|GetRoF))
  (Utilities|FlowControl|DoOnce false) ; enters at Reset
)

(event EventBeginPlay
  (|CallParentFunction) ; This node is disabled and will not be called.\nDrag off pins to build functionality.
)

(event Collision|EventActorBeginOverlap
  (params (OtherActor :type Actor%20Object%20Reference))
  (|CallParentFunction OtherActor) ; This node is disabled and will not be called.\nDrag off pins to build functionality.
)

(event EventTick
  (params (DeltaSeconds :type Float%20%28single-precision%29))
  (|CallParentFunction DeltaSeconds) ; This node is disabled and will not be called.\nDrag off pins to build functionality.
)

(event EventPullTrigger
  (bind _rof (Variables|Default|GetRoF))
  (Utilities|FlowControl|Sequence
    (:then_0
      (Utilities|FlowControl|DoOnce false :!label _label
        (:Completed
          (CallFunction|Proyectile 0.0 "/Game/Blueprints/DemWapons/Proyectiles/DamageBouncy.DamageBouncy_C")
          (Utilities|FlowControl|Delay _rof)
          (goto _label Reset))))
    (:then_1
      (bind _returnvalue (Utilities|Time|SetTimerbyEvent (delegate Custom|Fire) _rof true)))))

(event EventPullSecondary
  (bind _damage (Timeline|DiscoDamage PlayFromStart)
    (:Finished
      (Utilities|FlowControl|DoOnce false :!label _label
        (:Completed
          (bind _ref (CallFunction|Proyectile 0.0 "/Game/Blueprints/DemWapons/Proyectiles/Disco/DiscoSpawner.DiscoSpawner_C"))
          (bind _asdisco_spawner (Utilities|Casting|CastToDiscoSpawner _ref))
          (Variables|/Game/Blueprints/DemWapons/Proyectiles/Disco/DiscoSpawner.DiscoSpawner_C|SetDamage _asdisco_spawner (Math|Float|Truncate _damage))
          (Utilities|FlowControl|Delay 1.0)
          (goto _label Reset))))))

(event EventReleaseSecondary
  (Utilities|FlowControl|Sequence
    (:then_0
      (bind _damage (Timeline|DiscoDamage Stop)
        (:Finished
          _)))
    (:then_1
      _))
  (Utilities|FlowControl|DoOnce false :!label _label
    (:Completed
      (bind _ref (CallFunction|Proyectile 0.0 "/Game/Blueprints/DemWapons/Proyectiles/Disco/DiscoSpawner.DiscoSpawner_C"))
      (bind _asdisco_spawner (Utilities|Casting|CastToDiscoSpawner _ref))
      (Variables|/Game/Blueprints/DemWapons/Proyectiles/Disco/DiscoSpawner.DiscoSpawner_C|SetDamage _asdisco_spawner (Math|Float|Truncate _damage))
      (Utilities|FlowControl|Delay 1.0)
      (goto _label Reset))))

(event EventReleaseTrigger
  (Utilities|Time|ClearandInvalidateTimerbyHandle (stale EventPullTrigger _returnvalue)))

(fn ConstructionScript
  (|CallParentFunction))