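; Automatic projectile weapon Blueprint that fires bouncy projectiles repeatedly at its rate of fire.
; PullTrigger fires a first shot through a DoOnce, which resets after the rate-of-fire delay, and starts a looping timer at the same interval.
; The timer's Fire event re-enters the shot logic past the DoOnce, calling Proyectile with zero spread.
; Nothing in this graph clears the timer.
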(event Custom|Fire
  (CallFunction|Proyectile 0.0 "/Game/Blueprints/DemWapons/Proyectiles/Bouncy.Bouncy_C")
  (Utilities|FlowControl|Delay (Variables|Default|GetRoF))
  (Utilities|FlowControl|DoOnce false) ; enters at Reset
)

(event EventBeginPlay
  (|CallParentFunction) ; This node is disabled and will not be called.\nDrag off pins to build functionality.
)

(event Collision|EventActorBeginOverlap
  (params (OtherActor :type Actor%20Object%20Reference))
  (|CallParentFunction OtherActor) ; This node is disabled and will not be called.\nDrag off pins to build functionality.
)

(event EventTick
  (params (DeltaSeconds :type Float%20%28single-precision%29))
  (|CallParentFunction DeltaSeconds) ; This node is disabled and will not be called.\nDrag off pins to build functionality.
)

(event EventPullTrigger
  (bind _rof (Variables|Default|GetRoF))
  (Utilities|FlowControl|Sequence
    (:then_0
      (Utilities|FlowControl|DoOnce false :!label _label
        (:Completed
          (CallFunction|Proyectile 0.0 "/Game/Blueprints/DemWapons/Proyectiles/Bouncy.Bouncy_C")
          (Utilities|FlowControl|Delay _rof)
          (goto _label Reset))))
    (:then_1
      (Utilities|Time|SetTimerbyEvent (delegate Custom|Fire) _rof true))))

(fn ConstructionScript
  (|CallParentFunction))