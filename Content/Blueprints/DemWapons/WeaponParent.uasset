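; WeaponParent is a base weapon Blueprint with empty trigger, secondary, special and reload events, presumably for child weapons.
; BeginPlay caches the player and an ignore list of player and weapons.
; RayTrace and Proyectile trace from the camera within a spread cone, then spawn an effect or projectile at the muzzle Arrow, aimed at any hit.
; Damage is never applied; the enemy-hit check is disconnected and FireModeHandler is only a stub.
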(event Custom|PullTrigger)

(event Custom|ReleaseTrigger)

(event Custom|SpecialEffect)

(event Custom|Reload)

(event Custom|PullSecondary)

(event Custom|ReleaseSecondary)

(event EventBeginPlay
  (bind _outactors (Actor|GetAllActorsOfClass "/Game/Blueprints/PlayerBPs/PlayerBP.PlayerBP_C"))
  (Variables|Default|SetPlayer (Utilities|Array|Get(acopy) _outactors))
  (bind _outactors_2 (Actor|GetAllActorsOfClass "WeaponParent_C"))
  (bind _output_get (Variables|Default|SetIgnoreActors _outactors_2))
  (Utilities|Array|Add _output_get (Variables|Default|GetPlayer)))

(event Collision|EventActorBeginOverlap
  (params (OtherActor :type Actor%20Object%20Reference)))

(event EventTick
  (params (DeltaSeconds :type Float%20%28single-precision%29)))

(fn ConstructionScript)

(fn RayTrace
  (params (Range :type Integer) (Damage :type Integer) (Spread :type Float%20%28single-precision%29) (Effect :type Actor%20Class%20Reference))
  (bind _player (Variables|Default|GetPlayer))
  (bind _arrow (Variables|Default|GetArrow))
  (bind _returnvalue (Transformation|GetWorldLocation _arrow))
  (bind _camera (Variables|/Game/Blueprints/PlayerBPs/PlayerBP.PlayerBP_C|GetCamera _player))
  (bind (_outhit _returnvalue_2) (Collision|LineTraceByChannel (Transformation|GetWorldLocation _camera) (+ (* (Math|Random|RandomUnitVectorinConeinDegrees (Math|Vector|GetForwardVector (Transformation|GetWorldRotation _camera)) Spread) Range) (Transformation|GetWorldLocation (Variables|Default|GetArrow))) "TraceTypeQuery2" false (Variables|Default|GetIgnoreActors) "None" true "(R=1.000000,G=0.000000,B=0.000000,A=1.000000)" "(R=0.000000,G=1.000000,B=0.000000,A=1.000000)" 2.0))
  (if _returnvalue_2
    ;[1 1 1] Spawn muzzle effect
    (Game|SpawnActorfromClass Effect (Math|Transform|MakeTransform _returnvalue (Math|Rotator|FindLookatRotation _returnvalue (.location _outhit)) "1,1,1") "Undefined" 0 0)
    (else
      (Game|SpawnActorfromClass Effect (Math|Transform|MakeTransform _returnvalue (Transformation|GetWorldRotation (Variables|Default|GetArrow)) "1,1,1") "Undefined" 0 0))))

(fn FireModeHandler
  (params (Auto :type Boolean) (Range :type Integer) (Damage :type Integer) (Spread :type Float%20%28single-precision%29))
  (if Auto
    (Utilities|FlowControl|DoOnce false
      (:Completed
        (CallFunction|RayTrace Range Damage Spread)))))

(fn Proyectile
  (params (Spread :type Float%20%28single-precision%29) (Proyectile :type Actor%20Class%20Reference))
  (bind _player (Variables|Default|GetPlayer))
  (bind _arrow (Variables|Default|GetArrow))
  (bind _returnvalue (Transformation|GetWorldLocation _arrow))
  (bind _camera (Variables|/Game/Blueprints/PlayerBPs/PlayerBP.PlayerBP_C|GetCamera _player))
  (bind (_outhit _returnvalue_2) (Collision|LineTraceByChannel (Transformation|GetWorldLocation _camera) (+ (* (Math|Random|RandomUnitVectorinConeinDegrees (Math|Vector|GetForwardVector (Transformation|GetWorldRotation _camera)) Spread) 999999) (Transformation|GetWorldLocation (Variables|Default|GetArrow))) "TraceTypeQuery2" false (Variables|Default|GetIgnoreActors) "None" true "(R=1.000000,G=0.000000,B=0.000000,A=1.000000)" "(R=0.000000,G=1.000000,B=0.000000,A=1.000000)" 2.0))
  (if _returnvalue_2
    ;[1 1 1] Spawn proyectile
    (Game|SpawnActorfromClass Proyectile (Math|Transform|MakeTransform _returnvalue (Math|Rotator|FindLookatRotation _returnvalue (.location _outhit)) "1,1,1") "Undefined" 0 0)
    (else
      (Game|SpawnActorfromClass Proyectile (Math|Transform|MakeTransform _returnvalue (Transformation|GetWorldRotation _arrow) "1,1,1") "Undefined" 0 0))))