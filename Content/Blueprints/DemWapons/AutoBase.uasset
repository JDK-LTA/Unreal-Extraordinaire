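; Base Blueprint for automatic weapons that fire repeated ray-trace shots while the trigger is held.
; PullTrigger fires at once through a DoOnce that resets after the RoF delay, and starts a looping timer at the same interval.
; Each timer shot bypasses that gate to play the fire animation and call RayTrace with range, damage, spread and effect.
; ReleaseTrigger clears the timer.
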(event Custom|Fire
  (Components|Animation|PlayAnimation (Variables|Default|GetSkeletalMesh) "/Game/SciFiWeapDark/Weapons/Anims/Fire_Rifle_W.Fire_Rifle_W" false)
  (CallFunction|RayTrace (Variables|Default|GetRange) (Variables|Default|GetDamage) (Variables|Default|GetSpread) "/Game/Blueprints/DemWapons/Proyectiles/Effect.Effect_C")
  (Utilities|FlowControl|Delay (Variables|Default|GetRoF))
  (Utilities|FlowControl|DoOnce false) ; enters at Reset
)

(event EventBeginPlay
  (|CallParentFunction) ; This node is disabled and will not be called.\nDrag off pins to build functionality.
)

(event Collision|EventActorBeginOverlap
  (params (OtherActor :type Actor%20Object%20Reference))
  (|CallParentFunction OtherActor) ; This node is disabled and will not be called.\nDrag off pins to build functionality.
)

(event EventTick
  (params (DeltaSeconds :type Float%20%28single-precision%29))
  (|CallParentFunction DeltaSeconds) ; This node is disabled and will not be called.\nDrag off pins to build functionality.
)

(event EventReleaseTrigger
  (Utilities|Time|ClearandInvalidateTimerbyHandle (stale EventPullTrigger _returnvalue)))

(event EventPullTrigger
  (Utilities|FlowControl|Sequence
    (:then_0
      (Utilities|FlowControl|DoOnce false :!label _label
        (:Completed
          (Components|Animation|PlayAnimation (Variables|Default|GetSkeletalMesh) "/Game/SciFiWeapDark/Weapons/Anims/Fire_Rifle_W.Fire_Rifle_W" false)
          (CallFunction|RayTrace (Variables|Default|GetRange) (Variables|Default|GetDamage) (Variables|Default|GetSpread) "/Game/Blueprints/DemWapons/Proyectiles/Effect.Effect_C")
          (Utilities|FlowControl|Delay (Variables|Default|GetRoF))
          (goto _label Reset))))
    (:then_1
      (bind _returnvalue (Utilities|Time|SetTimerbyEvent (delegate Custom|Fire) (Variables|Default|GetRoF) true)))))

(fn ConstructionScript
  (|CallParentFunction))