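; AutoShot is an automatic shotgun weapon that fires bursts of spread ray traces while a trigger is held.
; Looping timers repeat each fire mode, with DoOnce and Delay gating the initial press against spam.
; Primary fire traces a fixed pellet count at the RoF interval.
; Secondary fire uses its own damage, spread and interval, growing its pellet count up to a cap whenever the burst's last trace returns true.
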(event Custom|FireSecondary
  (bind _bulletstoshoot (Variables|Default|GetBulletsToShoot))
  (Components|Animation|PlayAnimation (Variables|Default|GetSkeletalMesh) "/Game/SciFiWeapDark/Weapons/Anims/Fire_Shotgun_W.Fire_Shotgun_W" false)
  (for _index (range 0 (Variables|Default|GetBulletsToShoot))
    (bind _hit (CallFunction|RayTrace (Variables|Default|GetRange) (Variables|Default|GetRClickDamage) 25.0 "/Game/Blueprints/DemWapons/Proyectiles/Effect.Effect_C" "/Game/Sound/Shotgun/Shotgun_ImpactBody_Cue.Shotgun_ImpactBody_Cue" "/Game/Sound/Shotgun/Shotgun_ImpactSurface_Cue.Shotgun_ImpactSurface_Cue"))
    (Variables|Default|SetNewBullet (Math|Boolean|Equal(Boolean) _hit true)))
  (Utilities|FlowControl|Delay 0.2)
  (if (and (Variables|Default|GetNewBullet) (<= _bulletstoshoot 9))
    (Math|Integer|IncrementInt _bulletstoshoot
      (:%20%20
        _)))
  (Variables|Default|SetNewBullet false)
  (Utilities|FlowControl|DoOnce false) ; enters at Reset
)

(event Custom|Fire
  (Components|Animation|PlayAnimation (Variables|Default|GetSkeletalMesh) "/Game/SciFiWeapDark/Weapons/Anims/Fire_Shotgun_W.Fire_Shotgun_W" false)
  (for _index (range 0 10)
    (CallFunction|RayTrace (Variables|Default|GetRange) (Variables|Default|GetDamage) (Variables|Default|GetSpread) "/Game/Blueprints/DemWapons/Proyectiles/Effect.Effect_C" "/Game/Sound/Shotgun/Shotgun_ImpactBody_Cue.Shotgun_ImpactBody_Cue" "/Game/Sound/Shotgun/Shotgun_ImpactSurface_Cue.Shotgun_ImpactSurface_Cue"))
  (Utilities|FlowControl|Delay (Variables|Default|GetRoF))
  (Utilities|FlowControl|DoOnce false) ; enters at Reset
)

(event EventBeginPlay
  (|CallParentFunction) ; This node is disabled and will not be called.\nDrag off pins to build functionality.
)

(event Collision|EventActorBeginOverlap
  (params (OtherActor :type Actor%20Object%20Reference))
  (|CallParentFunction OtherActor) ; This node is disabled and will not be called.\nDrag off pins to build functionality.
)

(event EventReleaseSecondary
  (Utilities|Time|ClearandInvalidateTimerbyHandle (stale EventPullSecondary _returnvalue)))

(event EventTick
  (params (DeltaSeconds :type Float%20%28single-precision%29))
  (|CallParentFunction DeltaSeconds) ; This node is disabled and will not be called.\nDrag off pins to build functionality.
)

(event EventPullTrigger
  (Utilities|FlowControl|Sequence
    (:then_0
      (Utilities|FlowControl|DoOnce false :!label _label
        (:Completed
          (Components|Animation|PlayAnimation (Variables|Default|GetSkeletalMesh) "/Game/SciFiWeapDark/Weapons/Anims/Fire_Shotgun_W.Fire_Shotgun_W" false)
          (for _index (range 0 10)
            (CallFunction|RayTrace (Variables|Default|GetRange) (Variables|Default|GetDamage) (Variables|Default|GetSpread) "/Game/Blueprints/DemWapons/Proyectiles/Effect.Effect_C" "/Game/Sound/Shotgun/Shotgun_ImpactBody_Cue.Shotgun_ImpactBody_Cue" "/Game/Sound/Shotgun/Shotgun_ImpactSurface_Cue.Shotgun_ImpactSurface_Cue"))
          (Utilities|FlowControl|Delay (Variables|Default|GetRoF))
          (goto _label Reset))))
    (:then_1
      (bind _returnvalue (Utilities|Time|SetTimerbyEvent (delegate Custom|Fire) (Variables|Default|GetRoF) true)))))

(event EventReleaseTrigger
  (Utilities|Time|ClearandInvalidateTimerbyHandle (stale EventPullTrigger _returnvalue)))

(event EventPullSecondary
  (bind _bulletstoshoot (Variables|Default|GetBulletsToShoot))
  (Utilities|FlowControl|Sequence
    (:then_0
      (Utilities|FlowControl|DoOnce false :!label _label
        (:Completed
          (Components|Animation|PlayAnimation (Variables|Default|GetSkeletalMesh) "/Game/SciFiWeapDark/Weapons/Anims/Fire_Shotgun_W.Fire_Shotgun_W" false)
          (for _index (range 0 (Variables|Default|GetBulletsToShoot))
            (bind _hit (CallFunction|RayTrace (Variables|Default|GetRange) (Variables|Default|GetRClickDamage) 25.0 "/Game/Blueprints/DemWapons/Proyectiles/Effect.Effect_C" "/Game/Sound/Shotgun/Shotgun_ImpactBody_Cue.Shotgun_ImpactBody_Cue" "/Game/Sound/Shotgun/Shotgun_ImpactSurface_Cue.Shotgun_ImpactSurface_Cue"))
            (Variables|Default|SetNewBullet (Math|Boolean|Equal(Boolean) _hit true)))
          (Utilities|FlowControl|Delay 0.2)
          (if (and (Variables|Default|GetNewBullet) (<= _bulletstoshoot 9))
            (Math|Integer|IncrementInt _bulletstoshoot
              (:%20%20
                _)))
          (Variables|Default|SetNewBullet false)
          (goto _label Reset))))
    (:then_1
      (bind _returnvalue (Utilities|Time|SetTimerbyEvent (delegate Custom|FireSecondary) 0.2 true)))))

(fn ConstructionScript
  (|CallParentFunction))