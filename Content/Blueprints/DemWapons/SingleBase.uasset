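; Base Blueprint for a single-shot weapon that fires one hitscan shot per accepted trigger pull.
; PullTrigger plays the pistol fire animation on the skeletal mesh, then calls RayTrace with the weapon's range, damage, spread and effect variables.
; A DoOnce gate, reset after a delay set by RoF, ignores further pulls until that delay ends.
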(event EventBeginPlay
  (|CallParentFunction) ; This node is disabled and will not be called.\nDrag off pins to build functionality.
)

(event Collision|EventActorBeginOverlap
  (params (OtherActor :type Actor%20Object%20Reference))
  (|CallParentFunction OtherActor) ; This node is disabled and will not be called.\nDrag off pins to build functionality.
)

(event EventTick
  (params (DeltaSeconds :type Float%20%28single-precision%29))
  (|CallParentFunction DeltaSeconds) ; This node is disabled and will not be called.\nDrag off pins to build functionality.
)

(event EventPullTrigger
  (Utilities|FlowControl|DoOnce false :!label _label
    (:Completed
      (Components|Animation|PlayAnimation (Variables|Default|GetSkeletalMesh) "/Game/SciFiWeapDark/Weapons/Anims/Fire_Pistol_W.Fire_Pistol_W" false)
      (CallFunction|RayTrace (Variables|Default|GetRange) (Variables|Default|GetDamage) (Variables|Default|GetSpread) "/Game/Blueprints/DemWapons/Proyectiles/Effect.Effect_C")
      (Utilities|FlowControl|Delay (Variables|Default|GetRoF))
      (goto _label Reset))))

(fn ConstructionScript
  (|CallParentFunction))