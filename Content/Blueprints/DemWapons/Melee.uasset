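; Melee is a weapon Blueprint in the DemWapons folder that handles the player's melee attack.
; PullTrigger sets the Player's IsUsingMelee flag to true, waits 0.2 seconds, then clears it.
; The file contains no hit or damage logic of its own, and its BeginPlay, overlap and Tick events are disabled stubs.
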(event EventBeginPlay
  (|CallParentFunction) ; This node is disabled and will not be called.\nDrag off pins to build functionality.
)

(event Collision|EventActorBeginOverlap
  (params (OtherActor :type Actor%20Object%20Reference))
  (|CallParentFunction OtherActor) ; This node is disabled and will not be called.\nDrag off pins to build functionality.
)

(event EventTick
  (params (DeltaSeconds :type Float%20%28single-precision%29))
  (|CallParentFunction DeltaSeconds) ; This node is disabled and will not be called.\nDrag off pins to build functionality.
)

(event EventPullTrigger
  (bind _player (Variables|Default|GetPlayer))
  (Variables|/Game/Blueprints/PlayerBPs/PlayerBP.PlayerBP_C|SetisUsingMelee _player true)
  (Utilities|FlowControl|Delay 0.2)
  (Variables|/Game/Blueprints/PlayerBPs/PlayerBP.PlayerBP_C|SetisUsingMelee _player false))

(fn ConstructionScript
  (|CallParentFunction))